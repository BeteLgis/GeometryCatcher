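; BP_Shape is a falling collectible shape that the player catches in the Geometry Catcher game.
; Each Tick it moves down in world space by FallSpeed scaled with delta time, using a swept move.
; On overlap with BP_Player it reads the Color parameter from its mesh's dynamic material, passes it to GameManager.IncrementShapesCollected, then destroys itself.
; Collection only completes if material slot 0 holds a dynamic material instance.
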(event `self.ReceiveTick`
  (params (DeltaSeconds :type "Float (single-precision)"))
  (`self.K2_AddActorWorldOffset` (`KismetMathLibrary.MakeVector` 0.0 0.0 (* (* DeltaSeconds (`self.FallSpeed`)) -1.0)) true))

(event `self.ReceiveActorBeginOverlap`
  (params (OtherActor :type "Actor Object Reference"))
  (cast `/Game/GeometryCatcher/Blueprints/BP_Player` OtherActor)
  (bind _asmaterial_instance_dynamic (cast `MaterialInstanceDynamic` (`PrimitiveComponent.GetMaterial` (`self.StaticMesh`) 0)))
  (bind _returnvalue (`MaterialInstanceDynamic.K2_GetVectorParameterValue` _asmaterial_instance_dynamic "Color"))
  (`/Game/GeometryCatcher/Blueprints/BP_GameManager.Increment Shapes Collected` (`self.GameManager`) _returnvalue)
  (`self.K2_DestroyActor`))

(fn `UserConstructionScript`)